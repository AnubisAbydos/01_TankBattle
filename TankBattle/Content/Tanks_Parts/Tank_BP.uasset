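; Player-controllable tank Blueprint that drives, aims its camera and fires.
; On BeginPlay it hands the barrel and turret to TankAiming, and the left and right tracks to TankMovement.
; Move and turn axes feed TankMovement intents, while Fire calls TankAiming.
; Camera look splits yaw onto an azimuth gimbal and pitch onto the spring arm, both as local rotations by raw axis value.
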(event EventBeginPlay
  ;[1 1 1] Set Part References
  (Class|TankAimingComponent|Initialize (Variables|Default|GetTankAiming) (Variables|Default|GetBarrel) (Variables|Default|GetTankTurret))
  (Class|TankMovementComponent|Initialize (Variables|Default|GetTankMovement) (Variables|Default|GetLeft%20Track) (Variables|Default|GetRight%20Track)))

(event Input|ActionEvents|InputActionFire
  (params (Key :type Key%20Structure :default "AnyKey"))
  ;[1 1 1] Fire Shell Controls
  (:Pressed
    (Class|TankAimingComponent|Fire (Variables|Default|GetTankAiming))))

(event Input|AxisEvents|InputAxisAimAzimuth
  (params (AxisValue :type Float%20%28single-precision%29))
  ;[1 1 1] Camera Control
  (Transformation|AddLocalRotation (Variables|Default|GetAzimuth%20Gimbal) (Math|Rotator|MakeRotator 0.0 0.0 AxisValue) false false))

(event Input|AxisEvents|InputAxisLeftandRight
  (params (AxisValue :type Float%20%28single-precision%29))
  ;[1 1 1] Movement Control
  (Class|TankMovementComponent|IntendTurnRight (Variables|Default|GetTankMovement) AxisValue))

(event Input|AxisEvents|InputAxisAimElevation
  (params (AxisValue :type Float%20%28single-precision%29))
  ;[1 1 1] Camera Control
  (Transformation|AddLocalRotation (Variables|Default|GetSpringArm) (Math|Rotator|MakeRotator 0.0 AxisValue 0.0) false false))

(event Input|AxisEvents|InputAxisForwardandBackward
  (params (AxisValue :type Float%20%28single-precision%29))
  ;[1 1 1] Movement Control
  (Class|TankMovementComponent|IntendMoveForward (Variables|Default|GetTankMovement) AxisValue))

(fn ConstructionScript)